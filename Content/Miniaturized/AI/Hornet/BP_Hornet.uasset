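; BP_Hornet is the hornet enemy character, handling its health bar link and death sequence.
; On BeginPlay it registers itself as owner of its Hornet_HealthBar widget.
; Tick polls EnemyIsDead and, once, disables movement, plays a pose animation, waits briefly, sets CanDrop, then destroys the actor a tick later.
; UpdateWalkSpeed exposes a setter for the movement component's max walk speed.
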(event EventTick
  (params (DeltaSeconds :type Float%20%28single-precision%29))
  (if (Variables|Default|GetEnemyIsDead)
    (Utilities|FlowControl|DoOnce false
      (:Completed
        (Pawn|Components|CharacterMovement|DisableMovement (Variables|Character|GetCharacterMovement))
        (Components|Animation|PlayAnimation (Variables|Character|GetMesh) "/Game/Miniaturized/art_assets/characters/bee/animations/C_hornet_Anim_Armature_pose.C_hornet_Anim_Armature_pose" false)
        (Utilities|FlowControl|Delay 2.5)
        (Variables|Default|SetbCanDrop true)
        (Utilities|FlowControl|DelayUntilNextTick)
        (Actor|DestroyActor)))))

(event EventBeginPlay
  ;[1 1 1] Enemy health
  (bind _ashornet_health_bar (Utilities|Casting|CastToHornet_HealthBar (UserInterface|GetUserWidgetObject (Variables|Default|GetHealthBar))))
  (Variables|/Game/Miniaturized/AI/Hornet/Hornet_HealthBar.Hornet_HealthBar_C|SetHornetHealthBarOwner _ashornet_health_bar self))

(fn ConstructionScript)

(fn UpdateWalkSpeed
  (params (NewWalkSpeed :type Float%20%28double-precision%29))
  (Variables|/Script/Engine.CharacterMovementComponent|SetMaxWalkSpeed (Variables|Character|GetCharacterMovement) NewWalkSpeed))