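; Beetle enemy character that attacks the player and hands its behaviour to a behaviour tree.
; On begin play it links its health bar widget to itself, and pawn sensing sets the bSeenPlayer blackboard key on spotting the player.
; Hitting the player launches them and applies damage.
; Tick polls EnemyIsDead to run a one-time death animation, then briefly raises CanDrop before destroying the actor.
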(event OnSeePawn(BeetleSensing)
  (params (Pawn :type Pawn%20Object%20Reference))
  ;[1 1 1] Change value on blackboard to run different behaviour in behaviour tree
  (Utilities|Casting|CastToBP_PlayerCharacter Pawn)
  (AI|Components|Blackboard|SetValueasBool (AI|GetBlackboard (AI|GetAIController self)) (Utilities|Name|MakeLiteralName "bSeenPlayer") true))

(event EventTick
  (params (DeltaSeconds :type Float%20%28single-precision%29))
  ;[1 1 1] On death
  (if (Variables|Default|GetEnemyIsDead)
    (Utilities|FlowControl|DoOnce false
      (:Completed
        (Pawn|Components|CharacterMovement|DisableMovement (Variables|Character|GetCharacterMovement))
        (Components|Animation|PlayAnimation (Variables|Character|GetMesh) "/Game/Miniaturized/AI/Beetle/Animation/anime_Beetle_Death.anime_Beetle_Death" false)
        (Utilities|FlowControl|Delay 2.5)
        (Variables|Default|SetbCanDrop true)
        (Utilities|FlowControl|DelayUntilNextTick)
        (Actor|DestroyActor)))))

(event EventBeginPlay
  ;[1 1 1] Enemy health
  (bind _asbeetle_health_bar (Utilities|Casting|CastToBeetle_HealthBar (UserInterface|GetUserWidgetObject (Variables|Default|GetHealthbar))))
  (Variables|/Game/Miniaturized/AI/Beetle/Beetle_HealthBar.Beetle_HealthBar_C|SetBeetle_Owner _asbeetle_health_bar self))

(event Collision|EventHit
  (params (MyComp :type Primitive%20Component%20Object%20Reference) (Other :type Actor%20Object%20Reference) (OtherComp :type Primitive%20Component%20Object%20Reference) (bSelfMoved :type Boolean) (HitLocation :type Vector :default "0, 0, 0") (HitNormal :type Vector :default "0, 0, 0") (NormalImpulse :type Vector :default "0, 0, 0") (Hit :type Hit%20Result%20Structure%20%28by%20ref%29))
  ;[1 1 1] Deal damage to player
  (bind _asbp_player_character (Utilities|Casting|CastToBP_PlayerCharacter Other))
  (Character|LaunchCharacter _asbp_player_character "190.000000,190.000000,190.000000" false false)
  (Game|Damage|ApplyDamage _asbp_player_character 4.0 0 (stale OnSeePawn(BeetleSensing) Pawn)))

(fn ConstructionScript)