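; BP_Ant is an ant enemy character with a health bar widget and a death sequence.
; On BeginPlay it registers itself as the owner of its health bar widget.
; Tick watches EnemyIsDead, then once disables movement, plays the falling death animation, waits, raises CanDrop for a healing drop handled outside these graphs and destroys the actor.
; UpdateWalkSpeed sets the maximum walk speed.
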(event EventTick
  (params (DeltaSeconds :type Float%20%28single-precision%29))
  ;[1 1 1] Drop healing object after death
  (if (Variables|Default|GetEnemyIsDead)
    (Utilities|FlowControl|DoOnce false
      (:Completed
        (Pawn|Components|CharacterMovement|DisableMovement (Variables|Character|GetCharacterMovement))
        (Components|Animation|PlayAnimation (Variables|Character|GetMesh) "/Game/Miniaturized/AI/Ant/ABP_Ant_FallingDying_BS.ABP_Ant_FallingDying_BS" false)
        (Utilities|FlowControl|Delay 2.5)
        (Variables|Default|SetbCanDrop true)
        (Utilities|FlowControl|DelayUntilNextTick)
        (Actor|DestroyActor)))))

(event EventBeginPlay
  ;[1 1 1] Enemy health
  (bind _asant_health_bar (Utilities|Casting|CastToAnt_HealthBar (UserInterface|GetUserWidgetObject (Variables|Default|GetHealthBar))))
  (Variables|/Game/Miniaturized/AI/Ant/Ant_HealthBar.Ant_HealthBar_C|SetAnt_HealthBarOwner _asant_health_bar self))

(fn ConstructionScript)

(fn UpdateWalkSpeed
  (params (NewWalkSpeed :type Float%20%28double-precision%29))
  (Variables|/Script/Engine.CharacterMovementComponent|SetMaxWalkSpeed (Variables|Character|GetCharacterMovement) NewWalkSpeed))