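; Player character Blueprint that manages the health display and the switching menu.
; The open-menu input toggles the SwitchingMenu widget along with game pause, input mode and mouse cursor.
; Tick creates a new CharacterHealth widget every frame, adding it to the viewport while the menu is closed.
; With the menu open, Tick only hides a newly created widget, leaving those already on screen untouched.
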(event Input|EnhancedActionEvents|EnhancedInputActionIA_OpenMenu
  (params (ActionValue :type Boolean) (ElapsedSeconds :type Float%20%28double-precision%29) (TriggeredSeconds :type Float%20%28double-precision%29) (InputAction :type Input%20Action%20Object%20Reference :default "/Game/Miniaturized/Input/InputAction/IA_OpenMenu.IA_OpenMenu"))
  (bind _returnvalue (Game|GetPlayerController 0))
  ;[1 1 1] Display Menu
  (:Started
    (if (not (Variables|Default|GetbMenuIsOpen))
      (Variables|Default|SetbMenuIsOpen true)
      (bind _returnvalue_2 (UserInterface|CreateWidget "/Game/UI/SwitchingMenu.SwitchingMenu_C" _returnvalue))
      (bind _output_get (Variables|Default|SetMenu _returnvalue_2))
      (UserInterface|Viewport|AddtoViewport _output_get 0)
      (Input|SetInputModeGameandUI _returnvalue (Variables|Default|GetMenu) "DoNotLock" true false)
      (Variables|/Script/Engine.PlayerController|SetbShowMouseCursor (Game|GetPlayerController 0) true)
      (Game|SetGamePaused true)
      (else
        (Variables|Default|SetbMenuIsOpen false)
        (Widget|RemovefromParent (Variables|Default|GetMenu))
        (Game|SetGamePaused false)
        (Input|SetInputModeGameOnly _returnvalue false)
        (Variables|/Script/Engine.PlayerController|SetbShowMouseCursor (Game|GetPlayerController 0) false)))))

(event EventTick
  (params (DeltaSeconds :type Float%20%28single-precision%29))
  (bind _returnvalue (Game|GetPlayerController 0))
  ;[1 1 1] Display Progress bars, but hide it while menu is open
  (if (not (Variables|Default|GetbMenuIsOpen))
    (Variables|Default|SetbMenuIsOpen false)
    (bind _returnvalue_2 (UserInterface|CreateWidget "/Game/UI/CharacterHealth.CharacterHealth_C" _returnvalue))
    (UserInterface|Viewport|AddtoViewport _returnvalue_2 0)
    (else
      (Variables|Default|SetbMenuIsOpen true)
      (bind _returnvalue_3 (UserInterface|CreateWidget "/Game/UI/CharacterHealth.CharacterHealth_C" _returnvalue))
      (Widget|SetVisibility _returnvalue_3 "Hidden"))))

(fn ConstructionScript)